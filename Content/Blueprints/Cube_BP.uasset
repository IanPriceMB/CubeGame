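; Player cube pawn for an obstacle-dodging runner, scored by distance travelled along X.
; BeginPlay sets up Enhanced Input and the score HUD, then starts a looping timer that pushes the cube forward with impulses, while move input adds sideways impulses.
; Tick writes the score to the HUD.
; Obstacle hits or falloffworld stop the timer, set Canmove (which, despite its name, blocks steering) and reload the level after a delay.
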(event OnComponentHit(Cube)
  (params (HitComponent :type Primitive%20Component%20Object%20Reference) (OtherActor :type Actor%20Object%20Reference) (OtherComp :type Primitive%20Component%20Object%20Reference) (NormalImpulse :type Vector :default "0, 0, 0") (Hit :type Hit%20Result%20Structure%20%28by%20ref%29))
  (if (Actor|ActorHasTag OtherActor "Obstacle")
    (Variables|Default|Setcanmove? true)
    (Utilities|Time|ClearandInvalidateTimerbyHandle (Variables|Default|GetmoveForwardEvent))
    (Utilities|FlowControl|Delay (Variables|Default|GetDuration))
    (bind _returnvalue (Game|GetCurrentLevelName true))
    (Game|OpenLevel(byName) (Utilities|String|StringToName _returnvalue))))

(event Custom|Move%20Cube
  (Physics|AddImpulse (Variables|Default|GetCube) (Math|Vector|MakeVector (Variables|Default|Getforwardimpulse) 0.0 0.0) "None" true))

(event Custom|fall%20off%20world
  (Variables|Default|Setcanmove? true)
  (Utilities|Time|ClearandInvalidateTimerbyHandle (Variables|Default|GetmoveForwardEvent))
  (Utilities|FlowControl|Delay (Variables|Default|GetDuration))
  (bind _returnvalue (Game|GetCurrentLevelName true))
  (Game|OpenLevel(byName) (Utilities|String|StringToName _returnvalue)))

(event Input|EnhancedActionEvents|EnhancedInputActionMove_IA
  (params (ActionValue :type Float%20%28double-precision%29) (ElapsedSeconds :type Float%20%28double-precision%29) (TriggeredSeconds :type Float%20%28double-precision%29) (InputAction :type Input%20Action%20Object%20Reference :default "/Game/Input/Move_IA.Move_IA"))
  (if (not (Variables|Default|Getcanmove?))
    (Physics|AddImpulse (Variables|Default|GetCube) (Math|Vector|MakeVector 0.0 (* ActionValue (Variables|Default|GetTurnimpulse)) 0.0) "None" true)))

(event EventBeginPlay
  (bind _returnvalue (Game|GetPlayerController 0))
  (bind _asplayer_controller (Utilities|Casting|CastToPlayerController (Pawn|GetController)))
  (Utilities|IsValid (PlayerController|LocalPlayerSubsystems|GetEnhancedInputLocalPlayerSubsystem _asplayer_controller)
    (:Is%20Valid
      (Input|AddMappingContext (PlayerController|LocalPlayerSubsystems|GetEnhancedInputLocalPlayerSubsystem _asplayer_controller) "/Game/Input/Cube_IMC.Cube_IMC" 0 "(bIgnoreAllPressedKeysUntilRelease=True,bForceImmediately=False,bNotifyUserSettings=False)")
      (Variables|/Script/Engine.PlayerController|SetbShowMouseCursor _returnvalue false)
      (Input|SetInputModeGameOnly _returnvalue false)
      (bind _returnvalue_2 (UserInterface|CreateWidget "/Game/Blueprints/Score_WB.Score_WB_C"))
      (bind _output_get (Variables|Default|Setplayerhud _returnvalue_2))
      (UserInterface|Viewport|AddtoViewport _output_get 0)
      (bind _returnvalue_3 (Utilities|Time|SetTimerbyEvent (delegate Custom|Move%20Cube) 0.1 true))
      (Variables|Default|SetmoveForwardEvent _returnvalue_3))))

(event EventTick
  (params (DeltaSeconds :type Float%20%28single-precision%29))
  (bind _playerhud (Variables|Default|Getplayerhud))
  (Variables|Default|Setscore (Math|Float|Truncate (/ (.x (Transformation|GetWorldLocation (Variables|Default|GetCube))) 1e+02)))
  (Utilities|IsValid _playerhud
    (:Is%20Valid
      (Rendering|Components|TextRender|SetText (Variables|/Game/Blueprints/Score_WB.Score_WB_C|Getscoretext _playerhud) (Utilities|Text|ToText(Integer) (Variables|Default|Getscore))))))

(fn ConstructionScript)