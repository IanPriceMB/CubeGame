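; Level-completion trigger volume that ends the current level when the player's Cube_BP overlaps its Box component.
; On overlap, a Finallevel flag picks the outcome: a win widget leading to the main menu, or a level-beat widget leading to the next Level reference.
; Each branch shows its widget, waits briefly, then opens the target level by object reference.
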(event OnComponentBeginOverlap(Box)
  (params (OverlappedComponent :type Primitive%20Component%20Object%20Reference) (OtherActor :type Actor%20Object%20Reference) (OtherComp :type Primitive%20Component%20Object%20Reference) (OtherBodyIndex :type Integer) (bFromSweep :type Boolean) (SweepResult :type Hit%20Result%20Structure%20%28by%20ref%29))
  (Utilities|Casting|CastToCube_BP OtherActor)
  (if (Variables|Default|Getfinallevel)
    (bind _returnvalue (UserInterface|CreateWidget "/Game/Blueprints/win_WB.win_WB_C"))
    (UserInterface|Viewport|AddtoViewport _returnvalue 0)
    (Utilities|FlowControl|Delay 2.0)
    (Game|OpenLevel(byObjectReference) "/Game/Levels/MainMenu.MainMenu")
    (else
      (bind _returnvalue_2 (UserInterface|CreateWidget "/Game/Blueprints/levelbeat_WB.levelbeat_WB_C"))
      (UserInterface|Viewport|AddtoViewport _returnvalue_2 0)
      (Utilities|FlowControl|Delay 2.0)
      (Game|OpenLevel(byObjectReference) (Variables|Default|GetLevel)))))

(event EventBeginPlay)

(event Collision|EventActorBeginOverlap
  (params (OtherActor :type Actor%20Object%20Reference)))

(event EventTick
  (params (DeltaSeconds :type Float%20%28single-precision%29)))

(fn ConstructionScript)